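; Tree doodad actor that turns see-through while pawns are hidden behind it.
; Overlaps with the OpacityHelperBox component increment and decrement an occluded-pawn counter.
; TreeGraphics becomes transparent on the first overlap and opaque again only when the count returns to zero, so multiple overlapping pawns are handled correctly.
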(event OnComponentBeginOverlap(OpacityHelperBox)
  (params (OverlappedComponent :type Primitive%20Component%20Object%20Reference) (OtherActor :type Actor%20Object%20Reference) (OtherComp :type Primitive%20Component%20Object%20Reference) (OtherBodyIndex :type Integer) (bFromSweep :type Boolean) (SweepResult :type Hit%20Result%20Structure%20%28by%20ref%29))
  (bind _output_get (Variables|Default|SetOccludedPawnsCounter (+ (Variables|Default|GetOccludedPawnsCounter) 1)))
  (if (== _output_get 1)
    (Class|TreeGraphicsComponent|SetIsTransparent (Variables|Default|GetTreeGraphics) true)))

(event OnComponentEndOverlap(OpacityHelperBox)
  (params (OverlappedComponent :type Primitive%20Component%20Object%20Reference) (OtherActor :type Actor%20Object%20Reference) (OtherComp :type Primitive%20Component%20Object%20Reference) (OtherBodyIndex :type Integer))
  (if (> (Variables|Default|GetOccludedPawnsCounter) 0)
    (bind _output_get (Variables|Default|SetOccludedPawnsCounter (- (Variables|Default|GetOccludedPawnsCounter) 1)))
    (if (== _output_get 0)
      (Class|TreeGraphicsComponent|SetIsTransparent (Variables|Default|GetTreeGraphics) false))))

(event EventBeginPlay)

(event Collision|EventActorBeginOverlap
  (params (OtherActor :type Actor%20Object%20Reference)))

(event EventTick
  (params (DeltaSeconds :type Float%20%28single-precision%29)))

(fn ConstructionScript)