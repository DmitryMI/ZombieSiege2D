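; SurvivorFists is a weapon info Blueprint that defines a survivor's unarmed attack.
; The can-attack check passes when the 2D distance between the attacker's and target's simple collisions is within Range.
; The attack repeats that check, then sends the target a damage instance from the attacker with a random amount between the DamageMinMax bounds.
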(event EventBlueprintedCanAttackTarget
  (params (attacker :type Unit%20Base%20Object%20Reference) (target :type Unit%20Base%20Object%20Reference))
  (bind _returnvalue (Class|ZombieSiegeUtils|GetDistance2DBetweenSimpleCollisions attacker target))
  (Variables|Default|SetcanAttackTargetReturn (<= _returnvalue (Variables|Default|Getrange))))

(event EventBlueprintedAttackTarget
  (params (attacker :type Unit%20Base%20Object%20Reference) (target :type Unit%20Base%20Object%20Reference))
  (bind _damageminmax (Variables|Default|GetdamageMinMax))
  (bind (_x _y) (Math|Vector2D|BreakVector2D _damageminmax))
  (bind _returnvalue (Class|WeaponInfo|CanAttackTarget attacker target))
  (if _returnvalue
    (Class|UnitBase|ReceiveDamage target (Utilities|Struct|MakeDamageInstance attacker (Math|Random|RandomFloatinRange _x _y)))))