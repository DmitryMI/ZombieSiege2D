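; SurvivorRepair is a weapon info that acts as a repair, healing non-enemy targets at a Lumber cost.
; The can-attack check requires enough stored Lumber for the minimum damage value, a non-enemy target within range, and a Building classification on the attacker.
; Attacking calls ReceiveHealing with a zero amount and deducts the truncated returned value from the owner's Lumber.
; The random roll over the damage range is left unused.
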(event EventBlueprintedCanAttackTarget
  (params (attacker :type Unit%20Base%20Object%20Reference) (target :type Unit%20Base%20Object%20Reference))
  (bind _returnvalue (Class|ZombieSiegeUtils|GetDistance2DBetweenSimpleCollisions 0 target))
  (bind _returnvalue_2 (Class|UnitBase|GetOwningPlayerState attacker))
  (bind _returnvalue_3 (Class|ZombieSiegePlayerState|GetStoredResourceAmount _returnvalue_2 "Lumber"))
  (bind _returnvalue_4 (Class|WeaponInfo|GetDamageMinMax))
  (bind _returnvalue_5 (Class|ZombieSiegeUtils|AreEnemies attacker target))
  (bind _returnvalue_6 (Class|UnitBase|HasClassifications attacker "Building"))
  (Variables|Default|SetcanAttackTargetReturn (Math|Boolean|ANDBoolean (>= _returnvalue_3 (.X (Math|Vector2D|BreakVector2D _returnvalue_4))) (not _returnvalue_5) (<= _returnvalue (Variables|Default|Getrange)) _returnvalue_6)))

(event EventBlueprintedAttackTarget
  (params (attacker :type Unit%20Base%20Object%20Reference) (target :type Unit%20Base%20Object%20Reference))
  (bind _returnvalue (Class|WeaponInfo|CanAttackTarget attacker target))
  (if _returnvalue
    (bind _returnvalue_2 (Class|UnitBase|ReceiveHealing target (Utilities|Struct|MakeHealingInstance 0 0.0)))
    (bind _returnvalue_3 (Class|UnitBase|GetOwningPlayerState attacker))
    (Class|ZombieSiegePlayerState|TakeResourcefromStorage _returnvalue_3 "Lumber" (Math|Float|Truncate _returnvalue_2))))